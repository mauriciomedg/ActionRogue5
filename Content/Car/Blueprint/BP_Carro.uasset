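; BP_Carro is a drivable Chaos wheeled vehicle controlled through Enhanced Input.
; Input actions feed throttle, steering, brake and handbrake values to the vehicle movement component, while camera input drives controller pitch and yaw.
; The P key toggles the engine-start flag through a cast to SWheeledVehicleMovementComponent.
; BeginPlay sets the Chaos suspension slope threshold by console command, and debug prints show engine state and current gear.
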(event `Key|P`
  (params (Key :type "Key Structure"))
  (bind _engineonof (`self.EngineONOF`))
  (:`Pressed`
    (`/Engine/EditorBlueprintResources/StandardMacros.FlipFlop`
      (:`A`
        (set `self.EngineONOF` false))
      (:`B`
        (set `self.EngineONOF` true)))
    (bind _asswheeled_vehicle_movement_component (cast `SWheeledVehicleMovementComponent` (`self.VehicleMovementComponent`)))
    (`SWheeledVehicleMovementComponent.SetEngineStart` _asswheeled_vehicle_movement_component _engineonof)
    (`KismetSystemLibrary.PrintString` (`KismetStringLibrary.Concat_StrStr` "ENGINE START" (`KismetStringLibrary.Conv_BoolToString` _engineonof)))))

(event `self.ReceiveBeginPlay`
  (`KismetSystemLibrary.ExecuteConsoleCommand` "p.Chaos.Suspension.SlopeThreshold 1" null))

(event `EnhancedInput|/Game/Car/Inputs/IA_CameraMove`
  (params (ActionValue :type "Vector2D Structure") (ElapsedSeconds :type "Float (double-precision)") (TriggeredSeconds :type "Float (double-precision)") (InputAction :type "InputAction Object Reference" :default "/Game/Car/Inputs/IA_CameraMove.IA_CameraMove"))
  (:`Triggered`
    (`self.AddControllerPitchInput` ActionValue_Y)
    (`self.AddControllerYawInput` ActionValue_X)))

(event `EnhancedInput|/Game/Car/Inputs/IA_CarThrottle`
  (params (ActionValue :type "Float (double-precision)") (ElapsedSeconds :type "Float (double-precision)") (TriggeredSeconds :type "Float (double-precision)") (InputAction :type "InputAction Object Reference" :default "/Game/Car/Inputs/IA_CarThrottle.IA_CarThrottle"))
  (:`Triggered`
    (`ChaosVehicleMovementComponent.SetThrottleInput` (`self.VehicleMovementComponent`) ActionValue :!label _label))
  (:`Completed`
    (goto _label)))

(event `EnhancedInput|/Game/Car/Inputs/IA_CarSteering`
  (params (ActionValue :type "Float (double-precision)") (ElapsedSeconds :type "Float (double-precision)") (TriggeredSeconds :type "Float (double-precision)") (InputAction :type "InputAction Object Reference" :default "/Game/Car/Inputs/IA_CarSteering.IA_CarSteering"))
  (:`Triggered`
    (`ChaosVehicleMovementComponent.SetSteeringInput` (`self.VehicleMovementComponent`) ActionValue :!label _label_2))
  (:`Completed`
    (goto _label_2)))

(event `EnhancedInput|/Game/Car/Inputs/IA_Car_Brake`
  (params (ActionValue :type "Float (double-precision)") (ElapsedSeconds :type "Float (double-precision)") (TriggeredSeconds :type "Float (double-precision)") (InputAction :type "InputAction Object Reference" :default "/Game/Car/Inputs/IA_Car_Brake.IA_Car_Brake"))
  (:`Triggered`
    (`ChaosVehicleMovementComponent.SetBrakeInput` (`self.VehicleMovementComponent`) ActionValue :!label _label_3))
  (:`Completed`
    (goto _label_3)))

(event `EnhancedInput|/Game/Car/Inputs/IA_HandBrake`
  (params (ActionValue :type Boolean) (ElapsedSeconds :type "Float (double-precision)") (TriggeredSeconds :type "Float (double-precision)") (InputAction :type "InputAction Object Reference" :default "/Game/Car/Inputs/IA_HandBrake.IA_HandBrake"))
  (:`Triggered`
    (`ChaosVehicleMovementComponent.SetHandbrakeInput` (`self.VehicleMovementComponent`) ActionValue :!label _label_4))
  (:`Completed`
    (goto _label_4)))

(event `self.ReceiveTick`
  (params (DeltaSeconds :type "Float (single-precision)"))
  (`KismetSystemLibrary.PrintString` (`KismetStringLibrary.Conv_IntToString` (`ChaosVehicleMovementComponent.GetCurrentGear` (`self.VehicleMovementComponent`))) true true (struct :`G` 0.66 :`B` 1.0 :`A` 1.0) 0.0))

(fn `UserConstructionScript`)