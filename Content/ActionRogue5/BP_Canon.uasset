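; BP_Canon is a turret actor that tracks the player and fires magic projectiles at a fixed interval.
; A looping timer set on BeginPlay spawns a MagicProjectileBP at the cannon's own location and rotation.
; Each Tick rotates the whole actor to face the player's SCharacter, resetting its scale to one, with no range or line-of-sight check.
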(event `self.ReceiveBeginPlay`
  (`KismetSystemLibrary.K2_SetTimerDelegate` (delegate `OntimerElapsed`) 2.0 true))

(event `OntimerElapsed`
  (`|SpawnActorFromClass` "/Game/ActionRogue5/MagicProjectileBP.MagicProjectileBP_C" (`KismetMathLibrary.MakeTransform` (`self.K2_GetActorLocation`) (`self.K2_GetActorRotation`)) "Undefined" "MultiplyWithRoot" null null))

(event `self.ReceiveTick`
  (params (DeltaSeconds :type "Float (single-precision)"))
  (bind _returnvalue (`self.K2_GetActorLocation`))
  (bind _asscharacter (cast `SCharacter` (`GameplayStatics.GetPlayerPawn` 0)))
  (if true
    (`self.K2_SetActorTransform` (`KismetMathLibrary.MakeTransform` _returnvalue (`KismetMathLibrary.MakeRotFromX` (`KismetMathLibrary.Normal` (- (`self.K2_GetActorLocation` _asscharacter) _returnvalue)))))))

(fn `UserConstructionScript`)